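; Moving vehicle actor that drives a named military vehicle (Abrams tank or BTR-82 APC) along a geographic route on a Cesium globe.
; Initialize converts longitude/latitude points into a flattened spline, spawns the vehicle and starts movement.
; A timeline, rate-scaled to the path duration, moves and rotates it along the spline.
; Each update traces vertically for height, using hits on "globe"-tagged actors and otherwise zero.
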(event `LaunchVehicleMoving`
  (bind _spline (`self.Spline`))
  (`TimelineComponent.SetPlayRate` (`self.Move Vehicle T`) (/ 1.0 (`self.SecondsToCompletePath`)))
  (bind (_direction _movetrack) (`Timeline|Move Vehicle T`)
    (:`Update`
      (bind _returnvalue (`KismetMathLibrary.Lerp` 0.0 (`SplineComponent.GetSplineLength` (`self.Spline`)) _movetrack))
      (bind (_returnvalue_x _returnvalue_y) (`KismetMathLibrary.BreakVector` (`SplineComponent.GetLocationAtDistanceAlongSpline` _spline _returnvalue "World")))
      (bind (_outhit _returnvalue_2) (`KismetSystemLibrary.LineTraceSingle` (`KismetMathLibrary.MakeVector` _returnvalue_x _returnvalue_y 1000000000.0) (`KismetMathLibrary.MakeVector` _returnvalue_x _returnvalue_y) "TraceTypeQuery1" false (`|MakeArray` (`self.Vehicle`))))
      (`|ExecutionSequence`
        (:`then_0`
          (if _returnvalue_2
            (bind (_bblockinghit _binitialoverlap _time _distance _location _impactpoint _normal _impactnormal _physmat _hitactor) (`GameplayStatics.BreakHitResult` _outhit))
            (set `self.Calculated Z Altitude` (`KismetMathLibrary.SelectFloat` (.z _location) 0.0 (`self.ActorHasTag` _hitactor "globe")))
            (else
              (set `self.Calculated Z Altitude` 0.0))))
        (:`then_1`
          (`self.K2_SetActorTransform` (`self.Vehicle`) (`KismetMathLibrary.MakeTransform` (`KismetMathLibrary.MakeVector` _returnvalue_x _returnvalue_y (`self.Calculated Z Altitude`)) (`SplineComponent.GetRotationAtDistanceAlongSpline` _spline _returnvalue "Local")) false false))))))

(fn `Initialize`
  (bind _returnvalue (`CesiumGeoreference.GetDefaultGeoreference`))
  (set `self.Cesium Georeference Ref` _returnvalue)
  (`self.UpdateSplinePoints`))

(fn `SpawnVehicle`
  (`|ExecutionSequence`
    (:`then_0`
      (if (`KismetStringLibrary.EqualEqual_StrStr` (`self.MovingVehicleName`) "West_Tank_M1A1Abrams")
        (bind _returnvalue (`|SpawnActorFromClass` "/Game/VigilanteContent/Vehicles/West_Tank_M1A1Abrams/BP_West_Tank_M1A1Abrams.BP_West_Tank_M1A1Abrams_C" (`self.GetTransform`) "Undefined" "MultiplyWithRoot" null null))
        (set `self.Vehicle` _returnvalue)
        (`/Game/VigilanteContent/Vehicles/West_Tank_M1A1Abrams/BP_West_Tank_M1A1Abrams.SetWheelSmokeIntensity` _returnvalue 1.0)
        (`/Game/VigilanteContent/Vehicles/West_Tank_M1A1Abrams/BP_West_Tank_M1A1Abrams.SetSpeed` _returnvalue 100.0)
        (`/Game/VigilanteContent/Vehicles/West_Tank_M1A1Abrams/BP_West_Tank_M1A1Abrams.SetSpeed` _returnvalue 100.0)
        (elif (`KismetStringLibrary.EqualEqual_StrStr` (`self.MovingVehicleName`) "East_APC_BTR82")
          (bind _returnvalue_2 (`|SpawnActorFromClass` "/Game/VigilanteContent/Vehicles/East_APC_BTR82/BP_East_APC_BTR82.BP_East_APC_BTR82_C" (`self.GetTransform`) "Undefined" "MultiplyWithRoot" null null))
          (set `self.Vehicle` _returnvalue_2)
          (`/Game/VigilanteContent/Vehicles/East_APC_BTR82/BP_East_APC_BTR82.SetWheelSmokeIntensity` _returnvalue_2 1.0)
          (`/Game/VigilanteContent/Vehicles/East_APC_BTR82/BP_East_APC_BTR82.SetWheelSpeed` _returnvalue_2 100.0))))
    (:`then_1`
      (`self.LaunchVehicleMoving`))))

(fn `UpdateSplinePoints`
  (`SplineComponent.ClearSplinePoints` (`self.Spline`) true)
  (for _array_element (`self.PointCoordinates`)
    (bind (_returnvalue_x _returnvalue_y) (`KismetMathLibrary.BreakVector` (`CesiumGeoreference.TransformLongitudeLatitudeHeightToUnreal` (`self.Cesium Georeference Ref`) _array_element)))
    (`SplineComponent.AddSplinePoint` (`self.Spline`) (`KismetMathLibrary.MakeVector` _returnvalue_x _returnvalue_y) "World" true))
  (`self.SpawnVehicle`))

(fn `UserConstructionScript`)