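; BP_TankSpline builds a tank path spline that follows the Cesium globe surface, using longitude/latitude points from BP_OurScene.
; A one-second looping timer converts the points to Unreal space and traces vertically against "globe"-tagged actors for their height.
; Each pass rebuilds the spline from those positions.
; The timer clears itself once a pass finds every point unchanged, so clamping repeats until the terrain heights settle.
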(event `self.ReceiveBeginPlay`
  (bind _returnvalue (`GameplayStatics.GetActorOfClass` "/Game/BP_OurScene.BP_OurScene_C"))
  (set `self.BP Our Scene Ref` _returnvalue)
  (bind _returnvalue_2 (`CesiumGeoreference.GetDefaultGeoreference`))
  (set `self.Cesium Georeference Ref` _returnvalue_2)
  (bind _returnvalue_3 (`KismetSystemLibrary.K2_SetTimer` null "UpdateSplinePoints" 1.0 true))
  (set `self.TimerUpdateSplinePoints` _returnvalue_3))

(event `UpdateSplinePoints`
  (if (`self.bFinishClamping`)
    (`KismetSystemLibrary.K2_ClearAndInvalidateTimerHandle` (`self.TimerUpdateSplinePoints`))
    (else
      (`|ExecutionSequence`
        (:`then_0`
          (set `self.NumUnchangedPoints` 0)
          (bind _returnvalue (`OurScene.GetTankPathPoints` (`self.BP Our Scene Ref`)))
          (for (_array_element _array_index) _returnvalue
            (bind (_returnvalue_x _returnvalue_y) (`KismetMathLibrary.BreakVector` (`CesiumGeoreference.TransformLongitudeLatitudeHeightToUnreal` (`self.Cesium Georeference Ref`) _array_element)))
            (bind (_outhit _returnvalue_2) (`KismetSystemLibrary.LineTraceSingle` (`KismetMathLibrary.MakeVector` _returnvalue_x _returnvalue_y 1000000000.0) (`KismetMathLibrary.MakeVector` _returnvalue_x _returnvalue_y) "TraceTypeQuery1"))
            (if _returnvalue_2
              (bind (_bblockinghit _binitialoverlap _time _distance _location _impactpoint _normal _impactnormal _physmat _hitactor) (`GameplayStatics.BreakHitResult` _outhit))
              (if (`self.ActorHasTag` _hitactor "globe")
                (if (== (`KismetArrayLibrary.Array_Length` (`self.SplinePoints`)) (`KismetArrayLibrary.Array_Length` _returnvalue))
                  (bind _returnvalue_3 (`KismetMathLibrary.MakeVector` _returnvalue_x _returnvalue_y (.z _location)))
                  (if (`KismetMathLibrary.EqualExactly_VectorVector` _returnvalue_3 (`|GetArrayItem` (`self.SplinePoints`) _array_index))
                    (`/Engine/EditorBlueprintResources/StandardMacros.IncrementInt` (`self.NumUnchangedPoints`))
                    (else
                      (`KismetArrayLibrary.Array_Set` (`self.SplinePoints`) _array_index _returnvalue_3 true :!label _label)))
                  (else
                    (goto _label))))))
          (set `self.bFinishClamping` (== (`self.NumUnchangedPoints`) (`KismetArrayLibrary.Array_Length` _returnvalue))))
        (:`then_1`
          (`SplineComponent.ClearSplinePoints` (`self.Spline`) true)
          (for _array_element_2 (`self.SplinePoints`)
            (`SplineComponent.AddSplinePoint` (`self.Spline`) _array_element_2 "World" true)))))))

(fn `UserConstructionScript`)