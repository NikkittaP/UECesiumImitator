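; Drone camera view actor that flies a drone along a georeferenced spline and gives the operator a steerable camera.
; InitializeSpline builds a climb and waypoint route from lon/lat points, then LaunchDrone drives it by timeline.
; Tick feeds the compass widget and eases the camera toward nadir/forward targets, then holds world-space azimuth and elevation; manual input speed follows a zoom curve.
; Preset selection, coordinate tracking and auto zoom-out are empty stubs; the center-point trace result is unused.
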(event `self.ReceiveBeginPlay`
  (`|ExecutionSequence`
    (:`then_1`
      (bind _returnvalue (`|CreateWidget` "/Game/BP_CompassWidget.BP_CompassWidget_C"))
      (`UserWidget.AddToViewport` _returnvalue 0)
      (bind _output_get (set `self.CompassWidgetRef` _returnvalue))
      (`/Game/BP_CompassWidget.SetVariables` _output_get self))
    (:`then_2`)
    (:`then_3`)
    (:`then_4`)
    (:`then_5`)
    (:`then_6`)
    (:`then_7`)))

(event `self.ReceiveTick`
  (params (DeltaSeconds :type "Float (single-precision)"))
  (bind _compasswidgetref (`self.CompassWidgetRef`))
  ;[0.5843 0.1333 0.1333] EventTick
  (`|ExecutionSequence`
    (:`then_0`
      (`self.SetCurrentCameraFov`)
      (bind (_cameraazimuth _cameraelevation) (`self.CalculateCameraAzimuthAndPitch`))
      (`/Game/BP_CompassWidget.UpdateCompass` _compasswidgetref _cameraazimuth (`self.DroneHeading`))
      (`/Game/BP_CompassWidget.UpdatePitch` _compasswidgetref _cameraelevation))
    (:`then_1`
      (`self.CalculateCenterCoordinates`)
      (`self.Track Coordinate`))
    (:`then_2`
      ;;[1 1 1] Now it is always ON
      (if (`self.bAutoRotateCamera`)
        (if false
          (`SceneComponent.K2_SetRelativeRotation` (`self.Camera`) (`self.CurrentCameraRelativeRotation`) false false :!label _label)
          (else
            (`self.ProccessAutoRotateCameraToPreset` DeltaSeconds)))
        (else
          (goto _label))))))

(event `InputAxis|InputRotateCameraLeftRight`
  (params (AxisValue :type "Float (single-precision)"))
  (bind (_currentcamerarelativerotation_roll _currentcamerarelativerotation_pitch _currentcamerarelativerotation_yaw) (`KismetMathLibrary.BreakRotator` (`self.CurrentCameraRelativeRotation`)))
  ;[1 1 1] Rotate Camera
  (if (!= AxisValue 0.0)
    (set `self.bCameraAzimuthMovedByOperator` true)
    (set `self.CurrentCameraRelativeRotation` (`KismetMathLibrary.MakeRotator` 0.0 _currentcamerarelativerotation_pitch (+ (* AxisValue (* (`UECesiumImitatorGameInstance.GetRuntimeFloatCurveValue` (`self.CameraSpeedByZoomCurve`) (`self.CurrentCameraZoom`)) (`GameplayStatics.GetWorldDeltaSeconds`))) _currentcamerarelativerotation_yaw)))
    (else
      (set `self.bCameraAzimuthMovedByOperator` false))))

(event `LaunchDrone`
  (bind _spline (`self.Spline`))
  ;[1 1 1] Launch drone flight
  (`TimelineComponent.SetPlayRate` (`self.Move Drone T`) (/ 1.0 (`self.SecondsToCompletePath`)))
  (bind (_direction _movedrone) (`Timeline|Move Drone T`)
    (:`Update`
      (bind _returnvalue (`KismetMathLibrary.Lerp` 0.0 (`SplineComponent.GetSplineLength` (`self.Spline`)) _movedrone))
      (bind (_returnvalue_roll _returnvalue_pitch _returnvalue_yaw) (`KismetMathLibrary.BreakRotator` (`SplineComponent.GetRotationAtDistanceAlongSpline` _spline _returnvalue "Local")))
      (`SceneComponent.K2_SetWorldLocationAndRotation` (`self.Drone`) (`SplineComponent.GetLocationAtDistanceAlongSpline` _spline _returnvalue "World") (`KismetMathLibrary.MakeRotator` _returnvalue_roll 0.0 (+ _returnvalue_yaw 90.0)) false false))))

(event `InputAxis|InputRotateCameraUpDown`
  (params (AxisValue :type "Float (single-precision)"))
  (bind (_currentcamerarelativerotation_roll _currentcamerarelativerotation_pitch _currentcamerarelativerotation_yaw) (`KismetMathLibrary.BreakRotator` (`self.CurrentCameraRelativeRotation`)))
  ;[1 1 1] Rotate Camera
  (if (!= AxisValue 0.0)
    (set `self.bCameraElevationMovedByOperator` true)
    (bind _limitedcamerarelativerotation (`/Game/CommonLibraries.LimitCameraRelativeRotation` (`KismetMathLibrary.MakeRotator` 0.0 (+ (* AxisValue (* (`UECesiumImitatorGameInstance.GetRuntimeFloatCurveValue` (`self.CameraSpeedByZoomCurve`) (`self.CurrentCameraZoom`)) (`GameplayStatics.GetWorldDeltaSeconds`))) _currentcamerarelativerotation_pitch) _currentcamerarelativerotation_yaw)))
    (set `self.CurrentCameraRelativeRotation` _limitedcamerarelativerotation)
    (else
      (set `self.bCameraElevationMovedByOperator` false))))

(event `InputAxis|InputPresetCameraNadir`
  (params (AxisValue :type "Float (single-precision)"))
  ;[1 1 1] Rotate Camera
  (if (== AxisValue 1.0)
    (`self.RotateCameraToPreset` "NewEnumerator0")))

(event `InputAxis|InputPresetCameraForward`
  (params (AxisValue :type "Float (single-precision)"))
  ;[1 1 1] Rotate Camera
  (if (== AxisValue 1.0)
    (`self.RotateCameraToPreset` "NewEnumerator1")))

(fn `CalculateCameraAzimuthAndPitch`
  (returns (CameraAzimuth :type "Float (double-precision)") (CameraElevation :type "Float (double-precision)"))
  (bind (_returnvalue_roll _returnvalue_pitch _returnvalue_yaw) (`KismetMathLibrary.BreakRotator` (`SceneComponent.K2_GetComponentRotation` (`self.Drone`))))
  (bind _returnvalue (`SceneComponent.GetRelativeTransform` (`self.Camera`)))
  (bind _returnvalue_2 (+ _returnvalue_yaw (+ (.yaw (.rotation _returnvalue)) 90.0)))
  (bind _returnvalue_3 (`KismetMathLibrary.SelectFloat` (- _returnvalue_2 360.0) _returnvalue_2 (>= _returnvalue_2 360.0)))
  (set `self.DroneHeading` _returnvalue_yaw)
  (bind _output_get (set `self.DroneCameraHeading` (`KismetMathLibrary.SelectFloat` (+ _returnvalue_3 360.0) _returnvalue_3 (< _returnvalue_3 0.0))))
  (return _output_get (.pitch (.rotation _returnvalue))))

(fn `CalculateCenterCoordinates`
  (bind _camera (`self.Camera`))
  (bind _returnvalue (`SceneComponent.K2_GetComponentLocation` _camera))
  (bind _outactors (`GameplayStatics.GetAllActorsWithTag` "landscape"))
  (bind (_outhit _returnvalue_2) (`KismetSystemLibrary.LineTraceSingle` _returnvalue (+ _returnvalue (* (`SceneComponent.GetForwardVector` _camera) 100000000.0)) "TraceTypeQuery1" false _outactors))
  (if _returnvalue_2
    (if (`self.ActorHasTag` (`.HitActor` (`GameplayStatics.BreakHitResult` _outhit)) "globe")
      _)))

(fn `InitializeSpline`
  (locals (FlightLevel :type "Float (double-precision)"))
  (bind _returnvalue (`CesiumGeoreference.GetDefaultGeoreference`))
  (`SplineComponent.ClearSplinePoints` (`self.Spline`) true)
  (`SplineComponent.AddSplinePoint` (`self.Spline`) (`self.K2_GetActorLocation`) "World" true)
  (bind (_returnvalue_x _returnvalue_y _returnvalue_z) (`KismetMathLibrary.BreakVector` (`CesiumGeoreference.TransformUnrealToLongitudeLatitudeHeight` _returnvalue (`self.K2_GetActorLocation`))))
  (bind _returnvalue_2 (+ _returnvalue_z (`self.FlightAltitude`)))
  (set `local.FlightLevel` _returnvalue_2)
  (`SplineComponent.AddSplinePoint` (`self.Spline`) (`CesiumGeoreference.TransformLongitudeLatitudeHeightToUnreal` _returnvalue (`KismetMathLibrary.MakeVector` _returnvalue_x _returnvalue_y _returnvalue_2)) "World" true)
  (for _array_element (`self.PointCoordinates`)
    (`SplineComponent.AddSplinePoint` (`self.Spline`) (`CesiumGeoreference.TransformLongitudeLatitudeHeightToUnreal` _returnvalue (`KismetMathLibrary.MakeVector` (.x _array_element) (.y _array_element) (`local.FlightLevel`))) "World" true))
  (`SplineComponent.UpdateSpline` (`self.Spline`))
  (`self.LaunchDrone`))

(fn `ProccessAutoRotateCameraToPreset`
  (params (DeltaTime :type "Float (double-precision)"))
  (bind (_returnvalue_roll _returnvalue_pitch _returnvalue_yaw) (`KismetMathLibrary.BreakRotator` (`KismetMathLibrary.TransformRotation` (`self.GetTransform`) (`self.CurrentCameraRelativeRotation`))))
  (if (`|EnumEquality` (`self.CurrentCameraPreset`) "NewEnumerator2")
    ;[1 1 1] HoldYaw
    (`|ExecutionSequence`
      (:`then_0`
        (if (or (`self.bCameraAzimuthMovedByOperator`) (`self.bCameraElevationMovedByOperator`))
          (set `self.CameraHoldAzimuth` 999.0)
          (set `self.CameraHoldElevation` 999.0)))
      (:`then_1`
        (if (== (`self.CameraHoldAzimuth`) 999.0)
          (set `self.CameraHoldAzimuth` _returnvalue_yaw)))
      (:`then_2`
        (if (== (`self.CameraHoldElevation`) 999.0)
          (set `self.CameraHoldElevation` _returnvalue_pitch)))
      (:`then_3`
        (bind _returnvalue (`OurScene.InverseTransformRotationQuat` (`self.OurSceneInstanceRef`) (`self.GetTransform`) (`KismetMathLibrary.Conv_RotatorToQuaternion` (`KismetMathLibrary.MakeRotator` 0.0 (`self.CameraHoldElevation`) (`self.CameraHoldAzimuth`)))))
        (bind (_returnvalue_roll_2 _returnvalue_pitch_2 _returnvalue_yaw_2) (`KismetMathLibrary.BreakRotator` (`KismetMathLibrary.Quat_Rotator` _returnvalue)))
        (bind _limitedcamerarelativerotation (`/Game/CommonLibraries.LimitCameraRelativeRotation` (`KismetMathLibrary.MakeRotator` 0.0 _returnvalue_pitch_2 _returnvalue_yaw_2)))
        (bind _output_get (set `self.CurrentCameraRelativeRotation` _limitedcamerarelativerotation))
        (`SceneComponent.K2_SetRelativeRotation` (`self.Camera`) _output_get false false)))
    (elif (`|EnumEquality` (`self.CurrentCameraPreset`) "NewEnumerator0")
      (if (not (or (`self.bCameraAzimuthMovedByOperator`) (`self.bCameraElevationMovedByOperator`))) :!label _label
        (bind _output_get_2 (set `self.CurrentCameraRelativeRotation` (`KismetMathLibrary.RInterpTo` (`SceneComponent.RelativeRotation` (`self.Camera`)) (`self.TargetCameraRelativeRotation`) DeltaTime (`KismetMathLibrary.SelectFloat` 30.0 2.0 (`self.bFastCameraAutoRotate`)))))
        (`SceneComponent.K2_SetRelativeRotation` (`self.Camera`) _output_get_2 false false)
        (if (== _output_get_2 (`self.TargetCameraRelativeRotation`) :`ErrorTolerance` 0.1)
          (set `self.CameraHoldAzimuth` 999.0)
          (set `self.CameraHoldElevation` 999.0)
          (set `self.CurrentCameraPreset` "NewEnumerator2")))
      (elif (`|EnumEquality` (`self.CurrentCameraPreset`) "NewEnumerator1")
        (goto _label)
        (elif (`|EnumEquality` (`self.CurrentCameraPreset`) "NewEnumerator3")
          _)))))

(fn `ProccessAutoZoomOut`
  (params (DeltaTime :type "Float (double-precision)")))

(fn `RotateCameraToPreset`
  (params (CameraPreset :type "/Game/CameraPresets Enum" :default "NewEnumerator0") (OptionalToLocation :type "Vector Structure") (bFastRotate :type Boolean)))

(fn `SetCurrentCameraFov`
  (bind (_returnvalue_x _returnvalue_y) (`KismetMathLibrary.BreakVector2D` (`WidgetLayoutLibrary.GetViewportSize`)))
  (bind _fieldofview (`CameraComponent.FieldOfView` (`self.Camera`)))
  (set `self.CurrentHFOV` _fieldofview)
  (set `self.CurrentVFOV` (/ (* _returnvalue_y _fieldofview) _returnvalue_x)))

(fn `Track Coordinate`)

(fn `UserConstructionScript`)