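; BP_TestSpline is an actor that travels along the spline of a BP_TankSpline actor, starting on BeginPlay.
; It finds that actor by class and plays the Move timeline at a rate set by the inverse of TimeToCompleteMove.
; Each update maps the track value to a distance along the spline and sets the actor's transform from world-space location and local-space rotation at that point.
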(event `Move Tank`
  (bind _spline (`/Game/BP_TankSpline.Spline` (`self.TankSplineRef`)))
  (`TimelineComponent.SetPlayRate` (`self.Move`) (/ 1.0 (`self.TimeToCompleteMove`)))
  (bind (_direction _move_track) (`Timeline|Move`)
    (:`Update`
      (bind _returnvalue (`KismetMathLibrary.Lerp` 0.0 (`SplineComponent.GetSplineLength` (`/Game/BP_TankSpline.Spline` (`self.TankSplineRef`))) _move_track))
      (`self.K2_SetActorTransform` (`KismetMathLibrary.MakeTransform` (`SplineComponent.GetLocationAtDistanceAlongSpline` _spline _returnvalue "World") (`SplineComponent.GetRotationAtDistanceAlongSpline` _spline _returnvalue "Local"))))))

(event `self.ReceiveBeginPlay`
  (bind _returnvalue (`GameplayStatics.GetActorOfClass` "/Game/BP_TankSpline.BP_TankSpline_C"))
  (set `self.TankSplineRef` _returnvalue)
  (`self.Move Tank`))

(fn `UserConstructionScript`)