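; Actor that marks a target with a BP_TargetWidget held in its widget component, acting as a wrapper around that widget.
; Its functions forward size, distance, detection and tracking updates to the widget and return its position, size and distance.
; CheckHit projects the actor's location to screen space, rejects off-screen positions, and tests whether a given screen point lies inside the widget-sized square around it.
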(fn `CheckHit`
  (params (X :type "Float (double-precision)") (Y :type "Float (double-precision)"))
  (returns (bHit :type Boolean))
  (bind (_returnvalue_x _returnvalue_y) (`KismetMathLibrary.BreakVector2D` (`WidgetLayoutLibrary.GetViewportSize`)))
  (bind _screenlocation (`PlayerController.ProjectWorldLocationToScreen` (`GameplayStatics.GetPlayerController` 0) (`self.K2_GetActorLocation`) true))
  (bind _asbp_target_widget (cast `/Game/BP_TargetWidget` (`WidgetComponent.GetWidget` (`self.Widget`))))
  (if (or (or (< (`KismetMathLibrary.BreakVector2D` _screenlocation) 0.0) (> (`KismetMathLibrary.BreakVector2D` _screenlocation) _returnvalue_x)) (or (< (`.Y` (`KismetMathLibrary.BreakVector2D` _screenlocation)) 0.0) (> (`.Y` (`KismetMathLibrary.BreakVector2D` _screenlocation)) _returnvalue_y)))
    (return false)
    (else
      (bind _returnvalue (/ (`/Game/BP_TargetWidget.Size` _asbp_target_widget) 2.0))
      (return (and (and (< X (+ (`KismetMathLibrary.BreakVector2D` _screenlocation) _returnvalue)) (> X (- (`KismetMathLibrary.BreakVector2D` _screenlocation) _returnvalue))) (and (< Y (+ (`.Y` (`KismetMathLibrary.BreakVector2D` _screenlocation)) _returnvalue)) (> Y (- (`.Y` (`KismetMathLibrary.BreakVector2D` _screenlocation)) _returnvalue))))))))

(fn `DetectTarget`
  (params (bDetected :type Boolean))
  (bind _asbp_target_widget (cast `/Game/BP_TargetWidget` (`WidgetComponent.GetWidget` (`self.Widget`))))
  (`/Game/BP_TargetWidget.DetectTarget` _asbp_target_widget bDetected))

(fn `GetDistance`
  (returns (Distance :type "Float (double-precision)"))
  (bind _asbp_target_widget (cast `/Game/BP_TargetWidget` (`WidgetComponent.GetWidget` (`self.Widget`))))
  (return (`/Game/BP_TargetWidget.Distance` _asbp_target_widget)))

(fn `GetWidgetPositionAndSize`
  (returns (Position :type "Vector2D Structure") (Size :type "Vector2D Structure"))
  (bind _asbp_target_widget (cast `/Game/BP_TargetWidget` (`WidgetComponent.GetWidget` (`self.Widget`))))
  (bind (_position _size) (`/Game/BP_TargetWidget.GetWidgetPositionAndSize` _asbp_target_widget))
  (return _position _size))

(fn `TrackTarget`
  (params (bEnable :type Boolean))
  (bind _asbp_target_widget (cast `/Game/BP_TargetWidget` (`WidgetComponent.GetWidget` (`self.Widget`))))
  (`/Game/BP_TargetWidget.TrackTarget` _asbp_target_widget bEnable))

(fn `UpdateDistanceInfo`
  (params (DistanceToTarget :type "Float (double-precision)"))
  (bind _asbp_target_widget (cast `/Game/BP_TargetWidget` (`WidgetComponent.GetWidget` (`self.Widget`))))
  (`/Game/BP_TargetWidget.UpdateDistanceInfo` _asbp_target_widget DistanceToTarget))

(fn `UpdateTargetWidget`
  (params (Size :type "Float (double-precision)"))
  (bind _asbp_target_widget (cast `/Game/BP_TargetWidget` (`WidgetComponent.GetWidget` (`self.Widget`))))
  (`/Game/BP_TargetWidget.UpdateTargetWidget` _asbp_target_widget Size Size))

(fn `UserConstructionScript`)