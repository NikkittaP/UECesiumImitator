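; Scene controller for a drone-view simulation that spawns moving vehicles with target widgets and handles click-based target detection and lock-on.
; BeginPlay builds vehicles from path data and feeds flight plan points into BP_CameraView's spline.
; Tick resizes widgets by each object's screen radius.
; Clicks pick the nearest widget under the cursor, detecting new live vehicles or locking the drone camera, while double-clicking empty space clears the lock.
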(event `self.ReceiveBeginPlay`
  (`|ExecutionSequence`
    (:`then_0`
      (bind _returnvalue (`self.GetMovingVehiclesPathsPoints`))
      (for _array_element _returnvalue
        (bind _returnvalue_2 (`|SpawnActorFromClass` "/Game/BP_MovingVehicle.BP_MovingVehicle_C" (`self.GetTransform`) "Undefined" "MultiplyWithRoot" null null))
        (set `/Game/BP_MovingVehicle.MovingVehicleName` (break `MovingVehicleData` _array_element) _returnvalue_2)
        (set `/Game/BP_MovingVehicle.PointCoordinates` (`.PointCoordinates` (break `MovingVehicleData` _array_element)) _returnvalue_2)
        (set `/Game/BP_MovingVehicle.SecondsToCompletePath` (`.SecondsToCompletePath` (break `MovingVehicleData` _array_element)) _returnvalue_2)
        (`/Game/BP_MovingVehicle.Initialize` _returnvalue_2)
        ;[1 1 1] Add UI Widgets for each actor to highlight target
        (bind _returnvalue_3 (`|SpawnActorFromClass` "/Game/BP_TargetWidgetActor.BP_TargetWidgetActor_C" (`self.GetTransform` _returnvalue_2) "AlwaysSpawn" "OverrideRootScale" null null))
        (`self.K2_AttachToActor` _returnvalue_3 _returnvalue_2 "None" "SnapToTarget" "KeepRelative" "KeepRelative" true)
        (set `/Game/BP_MovingVehicle.TargetWidget` _returnvalue_3 _returnvalue_2)
        (`/Game/BP_TargetWidgetActor.DetectTarget` _returnvalue_3 false)))
    (:`then_1`
      (bind _returnvalue_4 (`self.GetFlightPlanPoints`))
      (bind _returnvalue_5 (`GameplayStatics.GetActorOfClass` "/Game/BP_CameraView.BP_CameraView_C"))
      (set `/Game/BP_CameraView.PointCoordinates` (`.PointCoordinates` (break `FlightPlanData` _returnvalue_4)) _returnvalue_5)
      (set `/Game/BP_CameraView.FlightAltitude` (break `FlightPlanData` _returnvalue_4) _returnvalue_5)
      (set `/Game/BP_CameraView.SecondsToCompletePath` (`.SecondsToCompletePath` (break `FlightPlanData` _returnvalue_4)) _returnvalue_5)
      (`/Game/BP_CameraView.InitializeSpline` _returnvalue_5))))

(event `self.ReceiveTick`
  (params (DeltaSeconds :type "Float (single-precision)"))
  (`self.ResizeTargetWidgets`))

(event `Key|LeftMouseButton`
  (params (Key :type "Key Structure"))
  ;[1 1 1] Mark target detected on click
  (:`Pressed`
    (set `self.NumTouches` (+ (`self.NumTouches`) 1)))
  (:`Released`
    (`|ExecutionSequence`
      (:`then_0`
        (`KismetSystemLibrary.Delay` 0.1)
        (if (>= (`self.NumTouches`) 2)
          (`self.SingleTap`)
          (if (`self.bShouldClearTarget`)
            (set `self.bShouldClearTarget` false)
            (`self.ClearPreviousTarget`)
            (`/Game/BP_CameraView.ClearLockOnTarget` (`self.DroneCameraView`)))
          (else
            (`self.SingleTap`))))
      (:`then_1`
        (`KismetSystemLibrary.Delay` 0.3)
        (set `self.NumTouches` 0)))))

(fn `ClearPreviousTarget`)

(fn `RedrawTargetIcon`
  (if (`self.bTargetDetected`)
    _
    (elif (!= (`self.SelectedActor`) null)
      (`self.ClearPreviousTarget`)
      (`/Game/BP_TargetWidgetActor.TrackTarget` (`self.SelectedActor`) true)
      (else
        (set `self.bShouldClearTarget` true)))))

(fn `ResizeTargetWidgets`
  (bind _asuecesium_imitator_game_instance (cast `UECesiumImitatorGameInstance` (`GameplayStatics.GetGameInstance`)))
  (bind _outactors (`GameplayStatics.GetAllActorsWithTag` "vehicle"))
  (bind _outactors_2 (`GameplayStatics.GetAllActorsWithTag` "target"))
  (`KismetArrayLibrary.Array_Append` _outactors _outactors_2)
  (for _array_element _outactors
    (bind _targetwidgetactor (`/Game/CommonLibraries.GetTargetWidgetActor` _array_element))
    (if (!= _targetwidgetactor null)
      (bind _returnvalue (`GameplayStatics.GetActorOfClass` "/Game/BP_CameraView.BP_CameraView_C"))
      (`/Game/BP_TargetWidgetActor.UpdateTargetWidget` _targetwidgetactor (`UECesiumImitatorGameInstance.GetObjectScreenRadius` _asuecesium_imitator_game_instance (`self.GetComponentByClass` _returnvalue "/Script/Engine.CameraComponent") _array_element)))))

(fn `SelectOrDetectTarget`
  (bind (_locationx _locationy) (`PlayerController.GetMousePosition` (`GameplayStatics.GetPlayerController` 0)))
  (bind _returnvalue (`self.GetAttachParentActor` (`self.SelectedActor`)))
  (set `self.SelectedActor` null)
  (set `self.ClosestDistance` 100000000.0)
  (`KismetArrayLibrary.Array_Clear` (`self.ActorsUnderTouch`))
  (bind _outactors (`GameplayStatics.GetAllActorsOfClass` "/Game/BP_TargetWidgetActor.BP_TargetWidgetActor_C"))
  (for _array_element _outactors
    (bind _bhit (`/Game/BP_TargetWidgetActor.CheckHit` _array_element _locationx _locationy))
    (if _bhit
      (`KismetArrayLibrary.Array_Add` (`self.ActorsUnderTouch`) _array_element)))
  (for _array_element_2 (`self.ActorsUnderTouch`)
    (bind _returnvalue_2 (`KismetMathLibrary.Vector_Distance` (`PlayerCameraManager.GetCameraLocation` (`GameplayStatics.GetPlayerCameraManager` 0)) (`self.K2_GetActorLocation` _array_element_2)))
    (if (< _returnvalue_2 (`self.ClosestDistance`))
      (set `self.ClosestDistance` _returnvalue_2)
      (set `self.SelectedActor` _array_element_2)))
  (if (!= (`self.SelectedActor`) null)
    (if (`self.ActorHasTag` _returnvalue "detected")
      _
      (elif (`self.ActorHasTag` _returnvalue "alive")
        (`/Game/CommonLibraries.DetectVehicle` (`self.GetAttachParentActor` (`self.SelectedActor`)))
        (set `self.bTargetDetected` true)))))

(fn `SingleTap`
  (set `self.bShouldClearTarget` false)
  (set `self.bTargetDetected` false)
  (`|ExecutionSequence`
    (:`then_0`
      (`self.SelectOrDetectTarget`))
    (:`then_1`
      (`self.RedrawTargetIcon`))
    (:`then_2`
      (if (`self.bTargetDetected`)
        _
        (elif (!= (`self.SelectedActor`) null)
          (set `self.PreviousSelectedActor` (`self.SelectedActor`))
          (`/Game/BP_CameraView.LockOnTarget` (`self.DroneCameraView`) false (`self.GetAttachParentActor` (`self.SelectedActor`))))))))

(fn `UserConstructionScript`)