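; Game mode that sets up the screen resolution and the WM Input Manager menu when play begins.
; BeginPlay runs a console command for fullscreen 1080p, adds the input manager smart menu widget, sets one player and starts the manager's UMG mode.
; Tick continually syncs the input manager's player count with the game's current player count.
; An unconnected GameUserSettings chain for windowed resolution never runs.
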(event `self.ReceiveBeginPlay`
  (bind _returnvalue (`WM_ControllerFunctionLib.Get_WM_InputManager`))
  (`|ExecutionSequence`
    (:`then_0`
      (`KismetSystemLibrary.ExecuteConsoleCommand` "r.setRes 1920x1080f" (`GameplayStatics.GetPlayerController` 0)))
    (:`then_1`
      (bind _returnvalue_2 (`|CreateWidget` "/WM_InputManager_Plugin/WM_UMG/WM_InputManagerSmartMenu.WM_InputManagerSmartMenu_C"))
      (`UserWidget.AddToViewport` _returnvalue_2 0)
      (`WM_InputManagerBase.SetNumberOfPlayers` _returnvalue 1)
      (`WM_InputManager.BeginUMG` _returnvalue))))

(event `self.ReceiveTick`
  (params (DeltaSeconds :type "Float (single-precision)"))
  ;[1 0.5412 0.9276] Sync PlayerNum
  (bind _returnvalue (`self.GetNumPlayers`))
  (`WM_InputManagerBase.SetNumberOfPlayers` (`WM_ControllerFunctionLib.Get_WM_InputManager`) _returnvalue))

(fn `UserConstructionScript`)